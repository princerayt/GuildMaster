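; BP_Calculations holds GameMode helper functions for warrior rest timers and for generating new mission tickets.
; Rest timers live in a GameMode map under unique keys, count down on each refresh, and are looked up by warrior index.
; The TimerOn flag tracks whether any timers remain.
; Mission generation picks random DB_MissionsTypes rows, rolls monster strength and booty, then refills and prints the mission selection widget's tickets.
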(fn `Create_NewMissionsTikets`
  (locals (WD_SelectMission :type "/Game/UI/WD_1_SelectMission Object Reference") (Booty :type Integer))
  (set `local.WD_SelectMission` (`/Game/BP/MainGameMode.WD_1_SelectMission` (`self.GameMode`)))
  (set `/Game/UI/WD_1_SelectMission.Array_NewMissions` (`|MakeArray`) (`local.WD_SelectMission`))
  (for _ (range 2)
    (bind _outrownames (`DataTableFunctionLibrary.GetDataTableRowNames` "/Game/Databases/StaticDatabases/DB_MissionsTypes.DB_MissionsTypes"))
    (bind _returnvalue (`|GetDataTableRow` "/Game/Databases/StaticDatabases/DB_MissionsTypes.DB_MissionsTypes" (`KismetArrayLibrary.Array_Random` _outrownames))
      (:`then`
        (bind (_missonname _minwarriorreputation _warriorsnum _monsterstrenght_min _monsterstrenght_max _terrain _reward _bootychance _booty_min _booty_max) (break `/Game/Databases/StaticDatabases/ST_MissionTypes` _returnvalue))
        (if (> _bootychance (`KismetMathLibrary.RandomIntegerInRange` 1 100))
          (set `local.Booty` 0)
          (else
            (set `local.Booty` (* (`KismetMathLibrary.RandomIntegerInRange` (/ _booty_min 10) (/ _booty_max 10)) 10))))
        (`KismetArrayLibrary.Array_Add` (`/Game/UI/WD_1_SelectMission.Array_NewMissions` (`local.WD_SelectMission`)) (make `/Game/Databases/ST_Mission` (`KismetTextLibrary.Conv_StringToText` _missonname) _minwarriorreputation (`KismetMathLibrary.RandomIntegerInRange` _monsterstrenght_min _monsterstrenght_max) _warriorsnum _reward (`KismetTextLibrary.Conv_StringToText` _terrain) 1.4 (`local.Booty`))))))
  (`/Game/UI/WD_1_SelectMission.Print_NewMissionsTickets` (`local.WD_SelectMission`)))

(fn `Timers_AddTimer`
  (params (WarriorIndex :type Integer))
  (bind _gamemode (`self.GameMode`))
  (bind _gamemode_2 (`self.GameMode`))
  (`BlueprintMapLibrary.Map_Add` (`/Game/BP/MainGameMode.Map_Timers` _gamemode) (`KismetStringLibrary.Concat_StrStr` "" (`KismetStringLibrary.Conv_IntToString` (`/Game/BP/MainGameMode.UniqNumber` _gamemode))) (make `/Game/Databases/ST_Timers` "WarriorRest" (`KismetStringLibrary.Concat_StrStr` "Warrior_" (`KismetStringLibrary.Conv_IntToString` WarriorIndex)) 60))
  (`/Engine/EditorBlueprintResources/StandardMacros.IncrementInt` (`/Game/BP/MainGameMode.UniqNumber` _gamemode_2)
    (:`  `
      (set `/Game/BP/MainGameMode.TimerOn` true _gamemode_2))))

(fn `Timers_GetTimeLeft`
  (params (TimerType :type String) (ObjectKey :type String) (WarriorIndex :type Integer))
  (returns (RestTimeText :type Text) (TimerOn :type Boolean))
  (locals (WarriorKey :type String) (WarriorIndexName :type String) (RestTime :type Integer))
  (bind _map_timers (`/Game/BP/MainGameMode.Map_Timers` (`self.GameMode`)))
  (bind (_timertype _objectindex _timebeforeoff) (break `/Game/Databases/ST_Timers` (`BlueprintMapLibrary.Map_Find` _map_timers (`local.WarriorKey`))))
  (set `local.WarriorIndexName` (`KismetStringLibrary.Concat_StrStr` "Warrior_" (`KismetStringLibrary.Conv_IntToString` WarriorIndex)))
  (set `local.RestTime` 0)
  (bind _keys (`BlueprintMapLibrary.Map_Keys` _map_timers))
  (for _array_element _keys
    (set `local.WarriorKey` _array_element)
    (if (`KismetStringLibrary.EqualEqual_StrStr` _timertype "WarriorRest")
      (if (`KismetStringLibrary.EqualEqual_StrStr` _objectindex (`local.WarriorIndexName`))
        (set `local.RestTime` _timebeforeoff))))
  (if (> (`local.RestTime`) 0)
    (return (`KismetTextLibrary.Conv_IntToText` (`local.RestTime`)) true)
    (else
      (return "" false))))

(fn `Timers_RefreshTimers`
  (locals (TimerName :type String))
  (bind _value (`BlueprintMapLibrary.Map_Find` (`/Game/BP/MainGameMode.Map_Timers` (`self.GameMode`)) (`local.TimerName`)))
  (bind ((`TimeBeforeOff_9_3C4E324E4299BA47A3DA3293A99DEEB7` _timebeforeoff)) (break `/Game/Databases/ST_Timers` _value))
  (bind _keys (`BlueprintMapLibrary.Map_Keys` (`/Game/BP/MainGameMode.Map_Timers` (`self.GameMode`))))
  (for _array_element _keys
    (set `local.TimerName` _array_element)
    (if (== _timebeforeoff 1)
      (`BlueprintMapLibrary.Map_Remove` (`/Game/BP/MainGameMode.Map_Timers` (`self.GameMode`)) (`local.TimerName`))
      (else
        (bind _structout (setmembers `/Game/Databases/ST_Timers` :`StructRef` _value :`TimeBeforeOff` (- _timebeforeoff 1)))
        (`BlueprintMapLibrary.Map_Add` (`/Game/BP/MainGameMode.Map_Timers` (`self.GameMode`)) (`local.TimerName`) _structout))))
  (if (== (`BlueprintMapLibrary.Map_Length` (`/Game/BP/MainGameMode.Map_Timers` (`self.GameMode`))) 0)
    (set `/Game/BP/MainGameMode.TimerOn` false (`self.GameMode`))))